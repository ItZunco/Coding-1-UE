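; BP_Potion is a holdable potion item that offers itself to BP_ThirdPersonCharacterCustom for pickup when that character overlaps its Sphere.
; Pickup attaches it to the parent mesh's hand_r socket, while Drop detaches it with flask physics simulation off and collision on.
; Primary and secondary actions consume it, clearing the character's HeldItem and destroying the actor.
; The HP and MP restoration is only printed text, with no stat changes.
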(event `self.Sphere.OnComponentBeginOverlap`
  (params (OverlappedComponent :type "PrimitiveComponent Object Reference") (OtherActor :type "Actor Object Reference") (OtherComp :type "PrimitiveComponent Object Reference") (OtherBodyIndex :type Integer) (bFromSweep :type Boolean) (SweepResult :type "HitResult Structure (by ref)"))
  (bind _asbp_third_person_character_custom (cast `/Game/Blueprints/BP_ThirdPersonCharacterCustom` OtherActor))
  (`/Game/Blueprints/BP_ThirdPersonCharacterCustom.TryToPickUp` _asbp_third_person_character_custom self))

(event `/Game/Blueprints/BPI_Item.Pickup`
  (params (ParentMesh :type "SkeletalMeshComponent Object Reference"))
  (`SceneComponent.K2_AttachToComponent` (`self.DefaultSceneRoot`) ParentMesh "hand_r" "SnapToTarget" "KeepRelative" "KeepRelative" true))

(event `/Game/Blueprints/BPI_Item.Drop`
  (`KismetSystemLibrary.PrintString` "You dropped the potion" true true (struct :`G` 0.66 :`B` 1.0 :`A` 1.0) 5.0)
  (`SceneComponent.K2_DetachFromComponent` (`self.DefaultSceneRoot`) "KeepRelative" "KeepRelative" "KeepRelative" true)
  (`PrimitiveComponent.SetSimulatePhysics` (`self.Flask Body`) false)
  (`PrimitiveComponent.SetCollisionEnabled` (`self.Flask Body`) "QueryAndPhysics"))

(event `/Game/Blueprints/BPI_Item.PrimaryAction`
  (params (Ref_ThirdPersonCharCustom :type "/Game/Blueprints/BP_ThirdPersonCharacterCustom Object Reference"))
  (`KismetSystemLibrary.PrintString` "The feeling of pain melted away... \nHP restored" true true (struct :`G` 1.0 :`B` 0.388586 :`A` 1.0) 5.0)
  (set `/Game/Blueprints/BP_ThirdPersonCharacterCustom.HeldItem` null Ref_ThirdPersonCharCustom)
  (`self.K2_DestroyActor`))

(event `/Game/Blueprints/BPI_Item.SecondaryAction`
  (params (Ref_ThirdPersonCharCustom :type "/Game/Blueprints/BP_ThirdPersonCharacterCustom Object Reference"))
  (`KismetSystemLibrary.PrintString` "Magical energy flows within you... \nMP restored" true true (struct :`R` 0.05725 :`B` 1.0 :`A` 1.0) 5.0)
  (set `/Game/Blueprints/BP_ThirdPersonCharacterCustom.HeldItem` null Ref_ThirdPersonCharCustom)
  (`self.K2_DestroyActor`))

(fn `UserConstructionScript`)