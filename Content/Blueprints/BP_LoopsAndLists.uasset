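; BP_LoopsAndLists is a demonstration actor that shows different loop styles through on-screen print messages.
; BeginPlay starts a Delay-paced endless game loop and a self-calling recursive event that counts, pauses, then resets and repeats.
; Tick reports its run count and frame time each frame.
; An input action runs a counted while loop within a single frame, contrasting with the latent, delayed loops.
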(event `self.ReceiveBeginPlay`
  (`KismetSystemLibrary.PrintString` "Loops and Lists is starting" true true (struct :`G` 0.66 :`B` 1.0 :`A` 1.0) 5.0)
  (`self.Simple Game Loop`)
  (`self.EnableInput` (`GameplayStatics.GetPlayerController` 0))
  (`self.Recursive Loop`))

(event `Simple Game Loop`
  (`KismetSystemLibrary.PrintString` "Starting Game Loop" true true (struct :`G` 0.133525 :`B` 1.0 :`A` 1.0) :!label _label)
  (`KismetSystemLibrary.Delay` 1.0) ; Wait One Second
  (goto _label))

(event `self.ReceiveTick`
  (params (DeltaSeconds :type "Float (single-precision)"))
  (bind _result (`/Engine/EditorBlueprintResources/StandardMacros.IncrementInt` (`self.Tick Counter`))
    (:`  `
      (`KismetSystemLibrary.PrintString` (`KismetStringLibrary.Concat_StrStr` "In event tick, we have run " (`KismetStringLibrary.Conv_IntToString` _result) "times.") true true (struct :`R` 0.927654 :`B` 1.0 :`A` 1.0) 0.0)
      (`KismetSystemLibrary.PrintString` (`KismetStringLibrary.Concat_StrStr` "The last frame took " (`KismetStringLibrary.Conv_DoubleToString` DeltaSeconds) "seconds to render.") true true (struct :`R` 0.087592 :`G` 0.4375 :`A` 1.0) DeltaSeconds))))

(event `InputAction|Start While Loop`
  (params (Key :type "Key Structure"))
  (bind _whileloopcounter (`self.WhileLoopCounter`))
  (:`Pressed`
    (`KismetSystemLibrary.PrintString` "Starting While Loop")
    (while (< (`self.WhileLoopCounter`) 25)
      (`/Engine/EditorBlueprintResources/StandardMacros.IncrementInt` _whileloopcounter
        (:`  `
          (`KismetSystemLibrary.PrintString` (`KismetStringLibrary.Concat_StrStr` "This while loop has run " (`KismetStringLibrary.Conv_IntToString` _whileloopcounter) "times.")))))
    (`KismetSystemLibrary.PrintString` "While Loop Complete")
    (set `self.WhileLoopCounter` 0) ; Reset Counter
  ))

(event `Recursive Loop`
  (if (< (`self.Recursion Counter`) 5)
    (bind _result (`/Engine/EditorBlueprintResources/StandardMacros.IncrementInt` (`self.Recursion Counter`))
      (:`  `
        (`KismetSystemLibrary.PrintString` (`KismetStringLibrary.Concat_StrStr` "Recursive Loops Ran:" (`KismetStringLibrary.Conv_IntToString` _result)) true true (struct :`R` 1.0 :`B` 0.274006 :`A` 1.0) 1.2)
        (`KismetSystemLibrary.Delay` 2.0)))
    (else
      (`KismetSystemLibrary.PrintString` "Resetting Recursive Loop")
      (set `self.Recursion Counter` 0)
      (`KismetSystemLibrary.Delay` 4.0)))
  (`self.Recursive Loop`) ; Starting event over again
)

(fn `UserConstructionScript`)